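; BP_Trampoline is a jump pad that bounces the player character upward when it overlaps the pad's box.
; It caches the player's BPC_EmbersEdge at BeginPlay and ignores other actors.
; A grounded player gets a temporarily raised JumpZVelocity and a JumpEvent call, with a hardcoded velocity restored after a short delay.
; A falling player is launched with vertical velocity overridden instead, and both paths play the jump pad sound.
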(event `self.ReceiveBeginPlay`
  (bind _asbpc_embers_edge (cast `/Game/EmbersEdge/Blueprints/GameBP/BPC_EmbersEdge` (`GameplayStatics.GetPlayerCharacter` 0)))
  (set `self.As BPC Embers Edge` _asbpc_embers_edge))

(event `self.Box.OnComponentBeginOverlap`
  (params (OverlappedComponent :type "PrimitiveComponent Object Reference") (OtherActor :type "Actor Object Reference") (OtherComp :type "PrimitiveComponent Object Reference") (OtherBodyIndex :type Integer) (bFromSweep :type Boolean) (SweepResult :type "HitResult Structure (by ref)"))
  (bind _as_bpc_embers_edge (`self.As BPC Embers Edge`))
  (bind _as_bpc_embers_edge_2 (`self.As BPC Embers Edge`))
  (if (== OtherActor _as_bpc_embers_edge_2)
    (if (not (`NavMovementComponent.IsFalling` (`Character.CharacterMovement` _as_bpc_embers_edge_2)))
      (set `CharacterMovementComponent.JumpZVelocity` 2000.0 (`Character.CharacterMovement` _as_bpc_embers_edge))
      (`/Game/EmbersEdge/Blueprints/GameBP/BPC_EmbersEdge.JumpEvent` _as_bpc_embers_edge)
      (`GameplayStatics.PlaySound2D` "/Game/EmbersEdge/SFX/Movement/SFX_JumpPad.SFX_JumpPad" 1.0 1.0 0.0 null null)
      (`KismetSystemLibrary.Delay` 0.2)
      (set `CharacterMovementComponent.JumpZVelocity` 800.0 (`Character.CharacterMovement` (`self.As BPC Embers Edge`)))
      (else
        (`Character.LaunchCharacter` (`self.As BPC Embers Edge`) (0.0 0.0 2000.0) false true)
        (`GameplayStatics.PlaySound2D` "/Game/EmbersEdge/SFX/Movement/SFX_JumpPad.SFX_JumpPad" 1.0 1.0 0.0 null null)))))

(fn `UserConstructionScript`)