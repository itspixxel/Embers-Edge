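; BP_SkullKey is a skull key pickup that the player character collects through an Interact event.
; Interact sets IsHoldingKey on the player's BPC_EmbersEdge character, then destroys the actor.
; BeginPlay caches that character, and two overlap spheres use it to toggle proximity billboards.
; Entering Sphere2 swaps Billboard for Billboard1, but leaving it only hides Billboard1 without restoring the first.
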(event `self.ReceiveBeginPlay`
  (bind _asbpc_embers_edge (cast `/Game/EmbersEdge/Blueprints/GameBP/BPC_EmbersEdge` (`GameplayStatics.GetPlayerCharacter` 0)))
  (set `self.CharacterRef` _asbpc_embers_edge))

(event `/Game/EmbersEdge/Blueprints/Interfaces/BPI_Interact.Interact`
  (bind _asbpc_embers_edge (cast `/Game/EmbersEdge/Blueprints/GameBP/BPC_EmbersEdge` (`GameplayStatics.GetPlayerCharacter` 0)))
  (bind _output_get (set `/Game/EmbersEdge/Blueprints/GameBP/BPC_EmbersEdge.bIsHoldingKey` true _asbpc_embers_edge))
  (if _output_get
    (`self.K2_DestroyActor`)
    (`KismetSystemLibrary.PrintString` "Player is holding key")
    (else
      (`KismetSystemLibrary.PrintString` "Key Grab Failed"))))

(event `self.Sphere1.OnComponentBeginOverlap`
  (params (OverlappedComponent :type "PrimitiveComponent Object Reference") (OtherActor :type "Actor Object Reference") (OtherComp :type "PrimitiveComponent Object Reference") (OtherBodyIndex :type Integer) (bFromSweep :type Boolean) (SweepResult :type "HitResult Structure (by ref)"))
  (if (== OtherActor (`self.CharacterRef`))
    (`SceneComponent.SetVisibility` (`self.Billboard`) true false)))

(event `self.Sphere1.OnComponentEndOverlap`
  (params (OverlappedComponent :type "PrimitiveComponent Object Reference") (OtherActor :type "Actor Object Reference") (OtherComp :type "PrimitiveComponent Object Reference") (OtherBodyIndex :type Integer))
  (if (== OtherActor (`self.CharacterRef`))
    (`SceneComponent.SetVisibility` (`self.Billboard`) false false)))

(event `self.Sphere2.OnComponentBeginOverlap`
  (params (OverlappedComponent :type "PrimitiveComponent Object Reference") (OtherActor :type "Actor Object Reference") (OtherComp :type "PrimitiveComponent Object Reference") (OtherBodyIndex :type Integer) (bFromSweep :type Boolean) (SweepResult :type "HitResult Structure (by ref)"))
  (if (== OtherActor (`self.CharacterRef`))
    (`SceneComponent.SetVisibility` (`self.Billboard1`) true false)
    (`SceneComponent.SetVisibility` (`self.Billboard`) false false)))

(event `self.Sphere2.OnComponentEndOverlap`
  (params (OverlappedComponent :type "PrimitiveComponent Object Reference") (OtherActor :type "Actor Object Reference") (OtherComp :type "PrimitiveComponent Object Reference") (OtherBodyIndex :type Integer))
  (if (== OtherActor (`self.CharacterRef`))
    (`SceneComponent.SetVisibility` (`self.Billboard1`) false false)))

(fn `UserConstructionScript`)