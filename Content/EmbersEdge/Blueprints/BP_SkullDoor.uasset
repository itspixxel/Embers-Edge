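; BP_SkullDoor is a barred door that opens and closes through OpenDoor and CloseDoor events.
; Each event checks IsOpen, then slides the SMBars mesh down to open or up to close with an eased, timed MoveComponentTo.
; Dust and an earthquake camera shake on the first player's controller run during the move, then stop as IsOpen updates.
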(event `OpenDoor`
  (bind _sm_bars (`self.SM_Bars`))
  (if (not (`self.IsOpen`))
    (`SceneComponent.SetVisibility` (`self.NS_Dust`) true false)
    (`PlayerController.ClientStartCameraShake` :`self` (`GameplayStatics.GetPlayerController` 0) :`Shake` "/Game/EmbersEdge/CameraShakes/CameraShake_Earthquake.CameraShake_Earthquake_C")
    (`KismetSystemLibrary.MoveComponentTo` (`self.SM_Bars`) (- (`SceneComponent.RelativeLocation` _sm_bars) (0.0 0.0 1200.0)) (`SceneComponent.RelativeRotation` _sm_bars) true true 2.0)
    (`PlayerController.ClientStopCameraShake` (`GameplayStatics.GetPlayerController` 0) null true)
    (`SceneComponent.SetVisibility` (`self.NS_Dust`) false false)
    (set `self.IsOpen` true)))

(event `CloseDoor`
  (bind _sm_bars (`self.SM_Bars`))
  (if (`self.IsOpen`)
    (`SceneComponent.SetVisibility` (`self.NS_Dust`) true false)
    (`PlayerController.ClientStartCameraShake` :`self` (`GameplayStatics.GetPlayerController` 0) :`Shake` "/Game/EmbersEdge/CameraShakes/CameraShake_Earthquake.CameraShake_Earthquake_C")
    (`KismetSystemLibrary.MoveComponentTo` (`self.SM_Bars`) (+ (`SceneComponent.RelativeLocation` _sm_bars) (0.0 0.0 1200.0)) (`SceneComponent.RelativeRotation` _sm_bars) true true 2.0)
    (`PlayerController.ClientStopCameraShake` (`GameplayStatics.GetPlayerController` 0) null true)
    (`SceneComponent.SetVisibility` (`self.NS_Dust`) false false)
    (set `self.IsOpen` false)))

(fn `UserConstructionScript`)