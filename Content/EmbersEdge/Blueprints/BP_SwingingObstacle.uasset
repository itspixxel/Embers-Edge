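; BP_SwingingObstacle is a hazard that swings continuously and ends the game when it touches the player character.
; Two alternating timelines loop from BeginPlay, lerping the root's relative pitch toward opposite sides to create the pendulum motion.
; Two box triggers check overlapping actors for the BPC_EmbersEdge class, then show the WBP_Lose widget and pause the game.
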(event `self.ReceiveBeginPlay`
  (`self.Swing`))

(event `Swing`
  (bind (_direction _alpha) (`Timeline|FirstSwingTimeline` :!via `PlayFromStart` :!label _label)
    (:`Update`
      (`SceneComponent.K2_SetRelativeRotation` (`self.DefaultSceneRoot`) (`KismetMathLibrary.MakeRotator` 0.0 (`KismetMathLibrary.Lerp` 0.0 30.0 _alpha)) false false))
    (:`Finished`
      (bind (_direction_2 _alpha_2) (`Timeline|SecondSwingTimeline` :!via `PlayFromStart`)
        (:`Update`
          (`SceneComponent.K2_SetRelativeRotation` (`self.DefaultSceneRoot`) (`KismetMathLibrary.MakeRotator` 0.0 (`KismetMathLibrary.Lerp` 0.0 -30.0 _alpha_2)) false false))
        (:`Finished`
          (goto _label :!via `PlayFromStart`))))))

(event `self.Box1.OnComponentBeginOverlap`
  (params (OverlappedComponent :type "PrimitiveComponent Object Reference") (OtherActor :type "Actor Object Reference") (OtherComp :type "PrimitiveComponent Object Reference") (OtherBodyIndex :type Integer) (bFromSweep :type Boolean) (SweepResult :type "HitResult Structure (by ref)"))
  (if (`KismetMathLibrary.ClassIsChildOf` (`GameplayStatics.GetObjectClass` OtherActor) "/Game/EmbersEdge/Blueprints/GameBP/BPC_EmbersEdge.BPC_EmbersEdge_C")
    (bind _returnvalue (`|CreateWidget` "/Game/EmbersEdge/UI/WBP_Lose.WBP_Lose_C" (`GameplayStatics.GetPlayerController` 0)))
    (`UserWidget.AddToViewport` _returnvalue 0)
    (`GameplayStatics.SetGamePaused` true)))

(event `self.Box.OnComponentBeginOverlap`
  (params (OverlappedComponent :type "PrimitiveComponent Object Reference") (OtherActor :type "Actor Object Reference") (OtherComp :type "PrimitiveComponent Object Reference") (OtherBodyIndex :type Integer) (bFromSweep :type Boolean) (SweepResult :type "HitResult Structure (by ref)"))
  (if (`KismetMathLibrary.ClassIsChildOf` (`GameplayStatics.GetObjectClass` OtherActor) "/Game/EmbersEdge/Blueprints/GameBP/BPC_EmbersEdge.BPC_EmbersEdge_C")
    (bind _returnvalue (`|CreateWidget` "/Game/EmbersEdge/UI/WBP_Lose.WBP_Lose_C" (`GameplayStatics.GetPlayerController` 0)))
    (`UserWidget.AddToViewport` _returnvalue 0)
    (`GameplayStatics.SetGamePaused` true)))

(fn `UserConstructionScript`)