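; BP_Door is an interactable door that the player knocks open with physics.
; Interact enables physics on the door, launches it with a strong impulse along the player's forward vector, makes it ignore Pawn collision and marks it open.
; Until then, two sphere triggers show billboard prompts to BPC_EmbersEdge characters, with Sphere swapping Sphere1's billboard for its own.
; End overlaps hide the billboards, though Sphere compares against a CharacterRef that is never assigned here.
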(event `/Game/EmbersEdge/Blueprints/Interfaces/BPI_Interact.Interact`
  (bind _door (`self.Door`))
  (`PrimitiveComponent.SetSimulatePhysics` _door true)
  (`PrimitiveComponent.AddImpulse` _door (* (`SceneComponent.GetForwardVector` (`Character.CapsuleComponent` (`GameplayStatics.GetPlayerCharacter` 0))) 250000.0) "None" false)
  (`PrimitiveComponent.SetCollisionResponseToChannel` (`self.Door`) "ECC_Pawn" "ECR_Ignore")
  (set `self.bIsOpen` true))

(event `self.Sphere1.OnComponentBeginOverlap`
  (params (OverlappedComponent :type "PrimitiveComponent Object Reference") (OtherActor :type "Actor Object Reference") (OtherComp :type "PrimitiveComponent Object Reference") (OtherBodyIndex :type Integer) (bFromSweep :type Boolean) (SweepResult :type "HitResult Structure (by ref)"))
  (if (`self.bIsOpen`)
    _
    (elif (`KismetMathLibrary.ClassIsChildOf` (`GameplayStatics.GetObjectClass` OtherActor) "/Game/EmbersEdge/Blueprints/GameBP/BPC_EmbersEdge.BPC_EmbersEdge_C")
      (`SceneComponent.SetVisibility` (`self.Billboard`) true false))))

(event `self.Sphere1.OnComponentEndOverlap`
  (params (OverlappedComponent :type "PrimitiveComponent Object Reference") (OtherActor :type "Actor Object Reference") (OtherComp :type "PrimitiveComponent Object Reference") (OtherBodyIndex :type Integer))
  (if (`KismetMathLibrary.ClassIsChildOf` (`GameplayStatics.GetObjectClass` OtherActor) "/Game/EmbersEdge/Blueprints/GameBP/BPC_EmbersEdge.BPC_EmbersEdge_C")
    (`SceneComponent.SetVisibility` (`self.Billboard`) false false)))

(event `self.Sphere.OnComponentBeginOverlap`
  (params (OverlappedComponent :type "PrimitiveComponent Object Reference") (OtherActor :type "Actor Object Reference") (OtherComp :type "PrimitiveComponent Object Reference") (OtherBodyIndex :type Integer) (bFromSweep :type Boolean) (SweepResult :type "HitResult Structure (by ref)"))
  (if (`self.bIsOpen`)
    _
    (elif (`KismetMathLibrary.ClassIsChildOf` (`GameplayStatics.GetObjectClass` OtherActor) "/Game/EmbersEdge/Blueprints/GameBP/BPC_EmbersEdge.BPC_EmbersEdge_C")
      (`SceneComponent.SetVisibility` (`self.Billboard1`) true false)
      (`SceneComponent.SetVisibility` (`self.Billboard`) false false))))

(event `self.Sphere.OnComponentEndOverlap`
  (params (OverlappedComponent :type "PrimitiveComponent Object Reference") (OtherActor :type "Actor Object Reference") (OtherComp :type "PrimitiveComponent Object Reference") (OtherBodyIndex :type Integer))
  (if (== OtherActor (`self.CharacterRef`))
    (`SceneComponent.SetVisibility` (`self.Billboard1`) false false)))

(fn `UserConstructionScript`)