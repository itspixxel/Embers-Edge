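; Interactable skull pedestal that acts as a key socket for a linked door in Ember's Edge.
; On interact, a player holding a key opens the referenced door, gives up the key and makes the pedestal's sphere visible.
; Otherwise, if the door is open, interacting closes it, returns the key to the player and hides the sphere.
; Key state lives as a flag on the player character, which is cached on BeginPlay.
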(event `self.ReceiveBeginPlay`
  (bind _asbpc_embers_edge (cast `/Game/EmbersEdge/Blueprints/GameBP/BPC_EmbersEdge` (`GameplayStatics.GetPlayerCharacter` 0)))
  (set `self.CharacterRef` _asbpc_embers_edge))

(event `/Game/EmbersEdge/Blueprints/Interfaces/BPI_Interact.Interact`
  (if (and (`/Game/EmbersEdge/Blueprints/GameBP/BPC_EmbersEdge.bIsHoldingKey` (`self.CharacterRef`)) (not (`/Game/EmbersEdge/Blueprints/BP_SkullDoor.bIsOpen` (`self.DoorRef`))))
    (`/Game/EmbersEdge/Blueprints/BP_SkullDoor.OpenDoor` (`self.DoorRef`))
    (set `/Game/EmbersEdge/Blueprints/GameBP/BPC_EmbersEdge.bIsHoldingKey` false (`self.CharacterRef`))
    (`SceneComponent.SetVisibility` (`self.Sphere`) true false)
    (elif (`/Game/EmbersEdge/Blueprints/BP_SkullDoor.bIsOpen` (`self.DoorRef`))
      (`/Game/EmbersEdge/Blueprints/BP_SkullDoor.CloseDoor` (`self.DoorRef`))
      (set `/Game/EmbersEdge/Blueprints/GameBP/BPC_EmbersEdge.bIsHoldingKey` true (`self.CharacterRef`))
      (`SceneComponent.SetVisibility` (`self.Sphere`) false false))))

(fn `UserConstructionScript`)